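; Pickup actor that gives the player a temporary attack speed boost and respawns after a delay.
; On overlap by an active Player-tagged actor, it plays the fire-rate pickup sound, shows a pickup widget and calls AttackSpeedBoost on the character with multiplier and duration.
; It then hides its mesh and deactivates, reappearing and reactivating after RespawnTime.
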(event `self.ReceiveBeginPlay`)

(event `self.ReceiveActorBeginOverlap`
  (params (OtherActor :type "Actor Object Reference"))
  (if (and (`self.ActorHasTag` OtherActor "Player") (`self.IsActive`))
    (bind _ascharacter_player (cast `/Game/Characters/Blueprints/Character_Player` OtherActor))
    (`GameplayStatics.PlaySoundAtLocation` (`/Game/Jeppe/Audio/SoundManager.PickupFiringrateSFX` (`/Game/Characters/Blueprints/Character_Player.SoundManager` _ascharacter_player)) (`self.K2_GetActorLocation` _ascharacter_player) (struct) 1.0 1.0 0.0 null null null)
    (bind _ascontroller_player (cast `/Game/Gameplay/Controller_Player` (`Pawn.GetController` _ascharacter_player)))
    (bind _returnvalue (`|CreateWidget` "/Game/Jeppe/HUD/Crosshair/OnASPickup.OnASPickup_C" _ascontroller_player))
    (`UserWidget.AddToPlayerScreen` _returnvalue 0)
    (`/Game/Characters/Blueprints/Character_Player.Attack Speed boost` _ascharacter_player (`self.AttackSpeedMultiplier`) (`self.BuffDuration`))
    (`SceneComponent.SetHiddenInGame` (`self.Mesh`) true true)
    (set `self.IsActive` false)
    (`KismetSystemLibrary.Delay` (`self.RespawnTime`))
    (`SceneComponent.SetHiddenInGame` (`self.Mesh`) false true)
    (set `self.IsActive` true)))

(fn `UserConstructionScript`)