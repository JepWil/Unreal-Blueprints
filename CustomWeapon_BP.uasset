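; CustomWeapon_BP is a projectile-style weapon actor that moves with ProjectileMovement and spins with RotatingMovement.
; Its first overlap, gated by DoOnce, activates the particle system, zeroes the projectile velocity and prints a debug message if the actor is tagged "Projectile".
; When projectile movement stops, the rotation is zeroed and the collision component switches to physics simulation.
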(event `self.ProjectileMovement.OnProjectileStop`
  (params (ImpactResult :type "HitResult Structure (by ref)"))
  (set `RotatingMovementComponent.RotationRate` (struct) (`self.RotatingMovement`))
  (`PrimitiveComponent.SetSimulatePhysics` (`self.Collision`) true))

(event `self.ReceiveActorBeginOverlap`
  (params (OtherActor :type "Actor Object Reference"))
  (`/Engine/EditorBlueprintResources/StandardMacros.DoOnce` false
    (:`Completed`
      (`ActorComponent.Activate` (`self.ParticleSystem`) false)
      (`ProjectileMovementComponent.SetVelocityInLocalSpace` (`self.ProjectileMovement`) (0.0 0.0 0.0))
      (if (`self.ActorHasTag` self "Projectile")
        (`KismetSystemLibrary.PrintString` "Has Tag")))))

(fn `UserConstructionScript`)