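; BP_HealthPowerUp is a respawning health pickup triggered when a Player-tagged Character_Player overlaps it.
; On pickup it plays a sound from the player's SoundManager, calls HealthPickup and sets Health to a fixed value.
; It then hides itself and deactivates Sphere1 for RespawnTimer before restoring both, with a DoOnce gate blocking repeat pickups until the respawn resets it.
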(event `self.ReceiveActorBeginOverlap`
  (params (OtherActor :type "Actor Object Reference"))
  (if (`self.ActorHasTag` OtherActor "Player")
    (bind _ascharacter_player (cast `/Game/Characters/Blueprints/Character_Player` OtherActor))
    (`/Engine/EditorBlueprintResources/StandardMacros.DoOnce` false :!label _label
      (:`Completed`
        (bind _soundmanager (`/Game/Characters/Blueprints/Character_Player.SoundManager` _ascharacter_player))
        (`GameplayStatics.PlaySoundAtLocation` (`/Game/Jeppe/Audio/SoundManager.PickupHealthSFX` _soundmanager) (`self.K2_GetActorLocation` _soundmanager) (struct) 1.0 1.0 0.0 null null null)
        (`/Game/Characters/Blueprints/Character_Player.Health pickup` _ascharacter_player)
        (set `/Game/Characters/Blueprints/Character_Player.Health` 1.25 _ascharacter_player)
        (`ActorComponent.SetActive` (`self.Sphere1`) false true)
        (`self.SetActorHiddenInGame` true)
        (`KismetSystemLibrary.Delay` (`self.RespawnTimer`))
        (`ActorComponent.SetActive` (`self.Sphere1`) true true)
        (`self.SetActorHiddenInGame` false)
        (goto _label :!via `Reset`)))))

(fn `UserConstructionScript`)