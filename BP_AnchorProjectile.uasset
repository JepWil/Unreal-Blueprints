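; Thrown anchor projectile that flies with optional homing, sticks to players it hits, and returns to its instigator's hand.
; Hits stop movement and show targeting particles scaled by camera distance.
; Recall is automatic after missing or a timed attachment, or player-pulled, which yanks attached players and flags the anchor as damaging.
; Return uses eased interpolation when far and velocity-compensated constant speed within close range until caught.
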(event `SetTargetSizeByDistance`
  (bind _returnvalue (`KismetMathLibrary.Conv_DoubleToVector` (* (`KismetMathLibrary.Sqrt` (`KismetMathLibrary.Vector_Distance` (`SceneComponent.K2_GetComponentLocation` (`GrappleManiaCharacter.FollowCamera` (`self.CastedInstigator`))) (`self.K2_GetActorLocation`))) 0.08)))
  (`/Engine/EditorBlueprintResources/StandardMacros.IsValid` (`self.CastedInstigator`)
    (:`Is Valid`
      (`SceneComponent.SetWorldScale3D` (`self.Targeting Particled Selected`) _returnvalue)
      (`SceneComponent.SetWorldScale3D` (`self.Targeting Particle`) _returnvalue))))

(event `SetTargetingParticle`
  (params (Selected :type Boolean))
  (bind _targeting_particle (`self.Targeting Particle`))
  (bind _targeting_particled_selected (`self.Targeting Particled Selected`))
  ;[1 1 1] Set Targeting particle
  (if (and (`self.Landed`) (not (`self.Recalled`)))
    (if (not (== Selected (`self.Selected`)))
      (set `self.Selected` Selected)
      (if Selected
        (`ActorComponent.SetActive` _targeting_particle false true)
        (`ActorComponent.SetActive` _targeting_particled_selected true true)
        (else
          (`ActorComponent.SetActive` _targeting_particle true true)
          (`ActorComponent.SetActive` _targeting_particled_selected false true))))))

(event `self.ReceiveHit`
  (params (MyComp :type "PrimitiveComponent Object Reference") (Other :type "Actor Object Reference") (OtherComp :type "PrimitiveComponent Object Reference") (bSelfMoved :type Boolean) (HitLocation :type "Vector Structure") (HitNormal :type "Vector Structure") (NormalImpulse :type "Vector Structure") (Hit :type "HitResult Structure (by ref)"))
  (bind (_bblockinghit _binitialoverlap _time _distance _location _impactpoint _normal _impactnormal _physmat _hitactor _hitcomponent _hitbonename) (`GameplayStatics.BreakHitResult` Hit))
  (bind _projectilemovement (`self.ProjectileMovement`))
  (bind _castedinstigator (`self.CastedInstigator`))
  ;[1 1 1] On hit
  (`self.K2_SetActorRotation` (`KismetMathLibrary.FindLookAtRotation` (`self.K2_GetActorLocation` (`self.GetInstigator`)) HitLocation) true)
  (`SceneComponent.K2_SetWorldLocation` (`self.Hit Particle`) _impactpoint false false)
  (`ActorComponent.SetActive` (`self.Hit Particle`) true true)
  (`ActorComponent.SetActive` (`self.Targeting Particle`) true true)
  (`ActorComponent.SetActive` (`self.Trail Particle`) false true)
  (`ProjectileMovementComponent.StopSimulating` _projectilemovement Hit)
  (`ActorComponent.SetActive` _projectilemovement false true)
  (set `self.Landed` true)
  (`PrimitiveComponent.IgnoreActorWhenMoving` (`self.Box`) (`self.GetInstigator`) false)
  (`PrimitiveComponent.SetCollisionResponseToAllChannels` (`self.Box`) "ECR_Overlap")
  (`PrimitiveComponent.SetCollisionResponseToChannel` (`self.Box`) "ECC_Visibility" "ECR_Block")
  (bind _ascharacter_player (cast `/Game/Characters/Blueprints/Character_Player` Other))
  (bind _output_get (set `self.AttachedToParent` _ascharacter_player))
  (if (`KismetStringLibrary.EqualEqual_StrStr` (`KismetStringLibrary.Conv_NameToString` _hitbonename))
    (`self.K2_AttachToActor` _output_get "None" "KeepWorld" "KeepWorld" "KeepRelative")
    (else
      (`self.K2_AttachToComponent` OtherComp _hitbonename "KeepWorld" "KeepWorld" "KeepWorld")))
  (set `self.AttachedToPlayer` true)
  (`PrimitiveComponent.IgnoreActorWhenMoving` (`self.Box`) _output_get true)
  (`/Game/Characters/Blueprints/Character_Player.TakeProjectileHit` _ascharacter_player self)
  (set `self.Damaging` false)
  (`KismetSystemLibrary.Delay` (`self.AttachedToPlayerAutoRecall`))
  (if (not (`self.Recalled`))
    (`/Game/Characters/Blueprints/Character_Player.RecallAnchor` _castedinstigator self false)
    (`/Engine/EditorBlueprintResources/StandardMacros.IncrementInt` (`/Game/Characters/Blueprints/Character_Player.MidAirAnchors` _castedinstigator))))

(event `RecallIfNotLandedAfter`
  (bind _castedinstigator (`self.CastedInstigator`))
  (if (not (`self.Landed`))
    (`/Game/Characters/Blueprints/Character_Player.RecallAnchor` _castedinstigator self false)
    (`/Engine/EditorBlueprintResources/StandardMacros.IncrementInt` (`/Game/Characters/Blueprints/Character_Player.MidAirAnchors` _castedinstigator))))

(event `CheckIfInstigatorIsDead`
  ;[1 1 1] Destroy this if player is dead
  (if (not (`KismetSystemLibrary.IsValid` (`self.GetInstigator`)))
    (if (not (`self.Landed`))
      (`KismetSystemLibrary.Delay` 3.0))
    (`self.K2_DestroyActor`)))

(event `CheckIfAttachedIsDead`
  ;[1 1 1] Destroy this if attached player is dead
  (if (`self.AttachedToPlayer`)
    (if (not (`KismetSystemLibrary.IsValid` (`self.AttachedToParent`)))
      (bind _ascharacter_player (cast `/Game/Characters/Blueprints/Character_Player` (`self.GetInstigator`)))
      (`/Game/Characters/Blueprints/Character_Player.RemoveAnchor` _ascharacter_player self))))

(event `self.ReceiveBeginPlay`
  (bind _returnvalue (`self.GetInstigator`))
  (bind _homingtarget (`self.HomingTarget`))
  (`KismetSystemLibrary.K2_SetTimerDelegate` (delegate `CheckIfInstigatorIsDead`) 1.0 true)
  (`KismetSystemLibrary.K2_SetTimerDelegate` (delegate `CheckIfAttachedIsDead`) 0.5 true)
  (`KismetSystemLibrary.K2_SetTimerDelegate` (delegate `RecallIfNotLandedAfter`) 1.0)
  (`KismetSystemLibrary.K2_SetTimerDelegate` (delegate `SetTargetSizeByDistance`) 0.02 true)
  (bind _ascharacter_player (cast `/Game/Characters/Blueprints/Character_Player` _returnvalue)
    (:`then`
      (set `self.CastedInstigator` _ascharacter_player)
      (`self.SetOwner` _returnvalue)
      (`PrimitiveComponent.IgnoreActorWhenMoving` (`self.Box`) (`self.GetInstigator`) true)
      (`ActorComponent.SetActive` (`self.Targeting Particled Selected`) false true)
      (`ActorComponent.SetActive` (`self.Targeting Particle`) false true)
      (`KismetSystemLibrary.Delay` 0.01)
      (`/Engine/EditorBlueprintResources/StandardMacros.IsValid` _homingtarget
        (:`Is Valid`
          (set `ProjectileMovementComponent.HomingTargetComponent` _homingtarget (`self.ProjectileMovement`)))))
    (:`CastFailed`
      (`KismetSystemLibrary.PrintString` "Projectile failed to cast instigator"))))

(event `self.Box.OnComponentBeginOverlap`
  (params (OverlappedComponent :type "PrimitiveComponent Object Reference") (OtherActor :type "Actor Object Reference") (OtherComp :type "PrimitiveComponent Object Reference") (OtherBodyIndex :type Integer) (bFromSweep :type Boolean) (SweepResult :type "HitResult Structure (by ref)"))
  (bind _castedinstigator (`self.CastedInstigator`))
  ;[1 1 1] Remove caught recalled anchor
  (if (and (== OtherActor (`self.GetInstigator`)) (`self.Recalled`))
    (`/Game/Characters/Blueprints/Character_Player.SetCaughtAnchor` _castedinstigator (`self.Damaging`))
    (`/Game/Characters/Blueprints/Character_Player.RemoveAnchor` _castedinstigator self)))

(event `Recall`
  (params (PulledByPlayer :type Boolean))
  (bind _projectilemovement (`self.ProjectileMovement`))
  ;[1 1 1] Recall
  (`/Engine/EditorBlueprintResources/StandardMacros.DoOnce` false
    (:`Completed`
      (`self.K2_DetachFromActor` "KeepRelative")
      (`ActorComponent.SetActive` (`self.Targeting Particled Selected`) false true)
      (`ActorComponent.SetActive` (`self.Targeting Particle`) false true)
      (`/Engine/EditorBlueprintResources/StandardMacros.IsValid` self
        (:`Is Valid`
          (`/Engine/EditorBlueprintResources/StandardMacros.IsValid` (`self.Box`)
            (:`Is Valid`
              (`/Engine/EditorBlueprintResources/StandardMacros.IsValid` (`self.StaticMesh`)
                (:`Is Valid`
                  (`ProjectileMovementComponent.StopSimulating` _projectilemovement (`GameplayStatics.MakeHitResult` false))
                  (`ActorComponent.SetActive` _projectilemovement false true)
                  (`PrimitiveComponent.SetCollisionResponseToChannel` (`self.Box`) "ECC_Pawn" "ECR_Overlap")
                  (`PrimitiveComponent.IgnoreActorWhenMoving` (`self.Box`) (`self.GetInstigator`) false)
                  (if PulledByPlayer
                    (set `self.Damaging` true)
                    (`BoxComponent.SetBoxExtent` (`self.Box`) (20.0 50.0 50.0) true)
                    (`SceneComponent.K2_SetRelativeLocation` (`self.StaticMesh`) (20.0 0.0 0.0) false false)
                    (if (`self.AttachedToPlayer`)
                      (`/Game/Characters/Blueprints/Character_Player.PullBackLaunch` (`self.AttachedToParent`) (`self.GetInstigator`)))
                    (`ActorComponent.SetActive` (`self.PassiveTrail Particle`) false true)
                    (`ActorComponent.SetActive` (`self.Trail Particle`) true true)
                    (else
                      (set `self.Damaging` false)
                      (`ActorComponent.SetActive` (`self.Trail Particle`) false true)
                      (`ActorComponent.SetActive` (`self.PassiveTrail Particle`) true true)))
                  (`KismetSystemLibrary.K2_SetTimerDelegate` (delegate `InterpolateAnchorToPlayer`) 0.02 true)
                  (set `self.AttachedToPlayer` false)
                  (`KismetSystemLibrary.Delay` 0.01)
                  (set `self.Recalled` true))
                (:`Is Not Valid`
                  (`/Game/Characters/Blueprints/Character_Player.RemoveAnchor` (`self.CastedInstigator`) self :!label _label))))
            (:`Is Not Valid`
              (goto _label))))
        (:`Is Not Valid`
          (goto _label))))))

(event `InterpolateAnchorToPlayer`
  (bind _returnvalue (`self.K2_GetActorLocation`))
  (bind _returnvalue_2 (`SceneComponent.GetSocketLocation` (`Character.Mesh` (`self.CastedInstigator`)) "Character1_RightHand_Socket"))
  ;[1 1 1] Recall
  (if (and (`KismetSystemLibrary.IsValid` (`self.GetInstigator`)) (`KismetSystemLibrary.IsValid` self))
    (if (<= (`KismetMathLibrary.Vector_Distance` _returnvalue _returnvalue_2) 500.0)
      (`SceneComponent.K2_SetWorldLocation` (`self.Box`) (`KismetMathLibrary.VInterpTo_Constant` _returnvalue _returnvalue_2 (`GameplayStatics.GetWorldDeltaSeconds`) (+ (`self.AnchorBaseRecallSpeed`) (`KismetMathLibrary.VSize` (`self.GetVelocity` (`self.CastedInstigator`))))) true false)
      (else
        (`SceneComponent.K2_SetWorldLocation` (`self.Box`) (`KismetMathLibrary.VInterpTo` _returnvalue _returnvalue_2 (`GameplayStatics.GetWorldDeltaSeconds`) (`self.AnchorInterpRecallSpeed`)) true false)))
    (`self.K2_SetActorRotation` (`KismetMathLibrary.FindLookAtRotation` (`self.K2_GetActorLocation`) (`self.K2_GetActorLocation` (`self.GetInstigator`))) true)))

(fn `StopColliding`)

(fn `UserConstructionScript`)