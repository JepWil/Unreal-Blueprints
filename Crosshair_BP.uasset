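; Crosshair_BP is a HUD Blueprint that builds the player's on-screen interface at BeginPlay.
; It creates crosshair, health/ammo, frag tracker, damage direction and anchor direction widgets for the owning player controller and adds them to that player's screen.
; It stores references to all but the frag tracker and clears the crosshair's OnKillActive flag.
; Tick, overlap and construction logic are empty.
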(event `self.ReceiveBeginPlay`
  (bind _returnvalue (`self.GetOwningPlayerController`))
  (bind _returnvalue_2 (`|CreateWidget` "/Game/Characters/Xhair/Xhair.Xhair_C" _returnvalue))
  (bind _output_get (set `self.XHairWidget` _returnvalue_2))
  (`UserWidget.AddToPlayerScreen` _output_get 0)
  (bind _returnvalue_3 (`|CreateWidget` "/Game/Jeppe/HUD/Widget_UI.Widget_UI_C" _returnvalue))
  (bind _output_get_2 (set `self.HealthAmmoWidget` _returnvalue_3))
  (`UserWidget.AddToPlayerScreen` _output_get_2 0)
  (bind _returnvalue_4 (`|CreateWidget` "/Game/Characters/Xhair/FragTrack.FragTrack_C" _returnvalue))
  (`UserWidget.AddToPlayerScreen` _returnvalue_4 0)
  (set `/Game/Characters/Xhair/Xhair.OnKillActive` false (`self.XHairWidget`))
  (bind _returnvalue_5 (`|CreateWidget` "/Game/UI/DamageDirectionIndicator/DamageDirectionIndicator.DamageDirectionIndicator_C" _returnvalue))
  (`UserWidget.AddToPlayerScreen` _returnvalue_5 0)
  (set `self.DamageDirectionWidget` _returnvalue_5)
  (bind _returnvalue_6 (`|CreateWidget` "/Game/UI/DamageDirectionIndicator/AnchorDirectionIndicator.AnchorDirectionIndicator_C" _returnvalue))
  (`UserWidget.AddToPlayerScreen` _returnvalue_6 0)
  (set `self.AnchorDirectionWidget` _returnvalue_6))

(event `self.ReceiveTick`
  (params (DeltaSeconds :type "Float (single-precision)")))

(fn `UserConstructionScript`)