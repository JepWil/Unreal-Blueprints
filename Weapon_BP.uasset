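; Weapon Blueprint that provides automatic fire while its trigger is held.
; PullTrigger passes a DoOnce gate, fires at once and starts a looping timer on the fire event at a rate set by RoundsPerSecond.
; Each shot spawns a Projectile_BP at the ProjectileSpawnPoint transform.
; ReleaseTrigger clears the timer and resets the gate for the next pull.
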(event `Pull Trigger`
  ;[1 1 1] Shoot Weapon
  (`/Engine/EditorBlueprintResources/StandardMacros.DoOnce` false :!label _label
    (:`Completed`
      (`self.Fire Projectile`)
      (`KismetSystemLibrary.K2_SetTimer` null "Fire Projectile" (/ 1.0 (`self.RoundsPerSecond`)) true))))

(event `Fire Projectile`
  ;[1 1 1] Shoot Weapon
  (`|SpawnActorFromClass` "/Game/Jeppe/Projectile/Projectile_BP.Projectile_BP_C" (`SceneComponent.K2_GetComponentToWorld` (`self.ProjectileSpawnPoint`)) "Undefined" "OverrideRootScale" null null))

(event `Release Trigger`
  ;[1 1 1] Shoot Weapon
  (`KismetSystemLibrary.K2_ClearTimer` null "Fire Projectile")
  (goto _label :!via `Reset`))

(fn `UserConstructionScript`)